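; Tank pawn Blueprint that handles player aiming and firing for a tank.
; On BeginPlay it passes its Turret and Barrel components to setter functions for later use.
; Aim axes orbit the camera by yawing an azimuth gimbal and pitching the spring arm separately.
; The Fire action calls a Fire function that is not defined in this graph.
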(event `self.ReceiveBeginPlay`
  (`self.SetTurretReference` (`self.Turret`))
  (`self.SetBarrelReference` (`self.Barrel`)))

(event `InputAxis|AimAzimuth`
  (params (AxisValue :type "Float (single-precision)"))
  ;[1 1 1] Camera Input setup
  (`SceneComponent.K2_AddLocalRotation` (`self.AzimuthGimbal`) (`KismetMathLibrary.MakeRotator` 0.0 0.0 AxisValue) false false))

(event `InputAxis|AimElevation`
  (params (AxisValue :type "Float (single-precision)"))
  ;[1 1 1] Camera Input setup
  (`SceneComponent.K2_AddLocalRotation` (`self.SpringArm`) (`KismetMathLibrary.MakeRotator` 0.0 AxisValue) false false))

(event `InputAction|Fire`
  (params (Key :type "Key Structure" :default "AnyKey"))
  ;[1 1 1] Camera Input setup
  (:`Pressed`
    (`self.Fire`)))

(fn `UserConstructionScript`)